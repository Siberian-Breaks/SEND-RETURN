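; Animated small concert speaker actor that plays a looping-style speaker animation at an adjustable play rate.
; On BeginPlay it stores Speed as Startspeed and overrides the skeletal mesh's animation data with the speaker animation at that rate.
; Tick compares Speed to Startspeed and, when they differ, calls PlayRateChange, which reruns the same setup so speed edits apply at runtime.
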(event Custom|PlayRateChange
  (Variables|Default|SetStartspeed (Variables|Default|GetSpeed))
  (Components|Animation|OverrideAnimationData (Variables|Default|GetSK_Speaker_Small) "/Game/ModularConcertStage/Meshes/Speakers_Rigged/SK_Speaker_Small_Anim.SK_Speaker_Small_Anim" true true 0.0 (Variables|Default|GetSpeed)))

(event EventBeginPlay
  (Variables|Default|SetStartspeed (Variables|Default|GetSpeed))
  (Components|Animation|OverrideAnimationData (Variables|Default|GetSK_Speaker_Small) "/Game/ModularConcertStage/Meshes/Speakers_Rigged/SK_Speaker_Small_Anim.SK_Speaker_Small_Anim" true true 0.0 (Variables|Default|GetSpeed)))

(event Collision|EventActorBeginOverlap
  (params (OtherActor :type Actor%20Object%20Reference)))

(event EventTick
  (params (DeltaSeconds :type Float%20%28single-precision%29))
  (if (not (== (Variables|Default|GetSpeed) (Variables|Default|GetStartspeed)))
    (CallFunction|PlayRateChange)))

(fn ConstructionScript)